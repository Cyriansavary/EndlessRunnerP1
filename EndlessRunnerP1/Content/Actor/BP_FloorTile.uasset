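; BP_FloorTile is a floor segment that fills itself with pickups or a hazard and signals when its end is reached.
; On BeginPlay, a weighted coin flip spawns either a random count of coins or one obstacle, using random classes and points within trigger bounds, attached to the tile.
; Overlapping EndPlatform fires the Exited dispatcher with the tile, and GetAttachTransfrom exposes the AttachPoint transform.
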(event OnComponentBeginOverlap(EndPlatform)
  (params (OverlappedComponent :type Primitive%20Component%20Object%20Reference) (OtherActor :type Actor%20Object%20Reference) (OtherComp :type Primitive%20Component%20Object%20Reference) (OtherBodyIndex :type Integer) (bFromSweep :type Boolean) (SweepResult :type Hit%20Result%20Structure%20%28by%20ref%29))
  (Default|CallExited self))

(event EventBeginPlay
  (if (Math|Random|RandomBoolwithWeight 0.6)
    (CallFunction|SpawnCoin)
    (else
      (CallFunction|SpawnObstacle))))

(fn ConstructionScript)

(fn GetAttachTransfrom
  (return (Transformation|GetWorldTransform (Variables|Default|GetAttachPoint))))

(fn SpawnObstacle
  (bind _triggerobstacle (Variables|Default|GetTriggerObstacle))
  (bind (_origin _boxextent) (Collision|GetComponentBounds _triggerobstacle))
  (bind _returnvalue (Game|SpawnActorfromClass (.OutItem (Utilities|Array|Random (Variables|Default|GetObstacle))) (Math|Transform|MakeTransform (Math|Random|RandomPointinBoundingBox _origin _boxextent) "0, 0, 0" "1.000000,1.000000,1.000000") "Undefined" "MultiplyWithRoot" 0 0))
  (Transformation|AttachActorToActor _returnvalue self "None" "KeepWorld" "KeepWorld" "KeepWorld" true))

(fn SpawnCoin
  (bind _triggercoin (Variables|Default|GetTriggerCoin))
  (bind (_origin _boxextent) (Collision|GetComponentBounds _triggercoin))
  (for _index (range 0 (Math|Random|RandomIntegerinRange 0 (Variables|Default|GetMaxCoin)))
    (bind _returnvalue (Game|SpawnActorfromClass (.OutItem (Utilities|Array|Random (Variables|Default|GetCoin))) (Math|Transform|MakeTransform (Math|Random|RandomPointinBoundingBox _origin _boxextent) "0, 0, 0" "1.000000,1.000000,1.000000") "Undefined" "MultiplyWithRoot" 0 0))
    (Transformation|AttachActorToActor _returnvalue self "None" "KeepWorld" "KeepWorld" "KeepWorld" true)))